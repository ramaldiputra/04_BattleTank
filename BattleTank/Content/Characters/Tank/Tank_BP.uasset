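; Tank Blueprint that wires up the barrel and turret and handles camera orbit and firing input.
; On BeginPlay it passes the barrel and turret components to setter functions defined outside these graphs and assigns the barrel mesh.
; Aim axes rotate an azimuth gimbal for yaw and the spring arm for pitch, scaled by delta time.
; The Fire action calls Fire, whose logic also lives outside these graphs.
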(event EventBeginPlay
  (bind _tankbarrel (Variables|Default|GetTankBarrel))
  (Class|Tank|SetBarrelReference _tankbarrel)
  (Class|Tank|SetTurretReference (Variables|Default|GetTurret))
  (Components|StaticMesh|SetStaticMesh _tankbarrel "/Game/Characters/Tank/tank_fbx_Barrel.tank_fbx_Barrel"))

(event Input|ActionEvents|InputActionFire
  (params (Key :type Key%20Structure :default "None"))
  ;[1 1 1] Camera Input Binding
  (:Pressed
    (Class|Tank|Fire)))

(event Input|AxisEvents|InputAxisAimAzimuth
  (params (AxisValue :type Float%20%28single-precision%29))
  ;[1 1 1] Camera Input Binding
  (Transformation|AddLocalRotation (Variables|Default|GetAzimuthGimbal) (Math|Rotator|MakeRotator 0.0 0.0 (* AxisValue (Utilities|Time|GetWorldDeltaSeconds) 1e+02)) false false))

(event Input|AxisEvents|InputAxisAimElevation
  (params (AxisValue :type Float%20%28single-precision%29))
  ;[1 1 1] Camera Input Binding
  (Transformation|AddLocalRotation (Variables|Default|GetSpringArm) (Math|Rotator|MakeRotator 0.0 (* AxisValue (Utilities|Time|GetWorldDeltaSeconds) 1e+02) 0.0) false false))

(fn ConstructionScript)